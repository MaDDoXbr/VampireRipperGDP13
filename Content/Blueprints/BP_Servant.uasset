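; BP_Servant is an AI pawn that detects and follows the player, using Pawn Sensing and a Blackboard.
; Seeing the player sets a "player seen" Blackboard bool, which a retriggerable delay clears once sightings stop.
; A move-to-player event re-issues AIMoveTo toward the player's location whether it succeeds or fails, forming a continuous chase.
; A FindValidPosNearby helper moves to a random navigable point within a given radius.
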(event `self.ReceiveBeginPlay`
  (set `self.PlayerPawn` (`GameplayStatics.GetPlayerPawn` 0))
  (set `self.BB` (`AIBlueprintHelperLibrary.GetBlackboard` (`AIBlueprintHelperLibrary.GetAIController` self))))

(event `self.PawnSensing.OnSeePawn`
  (params (Pawn :type "Pawn Object Reference"))
  (if (== Pawn (`self.PlayerPawn`))
    (`BlackboardComponent.SetValueAsBool` (`self.BB`) (`self.OnPlayerSeenKeyname`) true)
    (`KismetSystemLibrary.RetriggerableDelay` (`self.PlayerSeenRecheckDelay`))
    (`BlackboardComponent.SetValueAsBool` (`self.BB`) (`self.OnPlayerSeenKeyname`) false)))

(event `onMoveToPlayer`
  (`|AIMoveTo` self (`self.K2_GetActorLocation` (`self.PlayerPawn`)) null
    (:`OnSuccess`
      _)
    (:`OnFail`
      _))
  (`self.onMoveToPlayer`))

(event `self.ReceiveTick`
  (params (DeltaSeconds :type "Float (single-precision)")))

(fn `UserConstructionScript`)