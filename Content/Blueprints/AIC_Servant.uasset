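; AI controller for a servant character, which runs the BT_Servant behavior tree and feeds it the player's location.
; On BeginPlay it caches the first player's pawn, its own controlled pawn and the blackboard.
; Every Tick it writes the player pawn's location to the blackboard key named by the KeyName variable.
; The cached controlled pawn is not used elsewhere in this graph.
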(event `self.ReceiveBeginPlay`
  (set `self.PlayerPawn` (`GameplayStatics.GetPlayerPawn` 0))
  (set `self.ControlledPawn` (`self.K2_GetPawn`))
  (`self.RunBehaviorTree` "/Game/AI/BT_Servant.BT_Servant")
  (set `self.BB` (`AIBlueprintHelperLibrary.GetBlackboard` null)))

(event `self.ReceiveTick`
  (params (DeltaSeconds :type "Float (single-precision)"))
  (`BlackboardComponent.SetValueAsVector` (`self.BB`) (`self.Key Name`) (`self.K2_GetActorLocation` (`self.PlayerPawn`))))

(fn `UserConstructionScript`)