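; BP_Servant is an AI-controlled servant character that senses the player and can move toward them or wander nearby.
; Pawn sensing sets PlayerInSight, and a retriggerable delay clears it when sightings stop, sending a player-lost event to the StateTree.
; The move-to-player event re-calls itself after every success or failure, while FindValidPosNearby moves to a random navigable point.
; Older Blackboard-based sight logic remains disconnected.
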(event `self.ReceiveBeginPlay`
  (set `self.PlayerPawn` (`GameplayStatics.GetPlayerPawn` 0))
  (set `self.BB` (`AIBlueprintHelperLibrary.GetBlackboard` (`AIBlueprintHelperLibrary.GetAIController` self))))

(event `self.PawnSensing.OnSeePawn`
  (params (Pawn :type "Pawn Object Reference"))
  (if (== Pawn (`self.PlayerPawn`))
    (set `self.bPlayerInSight` true)
    (`KismetSystemLibrary.RetriggerableDelay` (`self.PlayerSeenRecheckDelay`))
    (set `self.bPlayerInSight` false)
    (`StateTreeComponent.SendStateTreeEvent` (`self.StateTree`) (`self.PlayerLost Event`))
    (`KismetSystemLibrary.PrintString` "Lost Player...")))

(event `self.ReceiveTick`
  (params (DeltaSeconds :type "Float (single-precision)")))

(event `onMoveToPlayer`
  (`|AIMoveTo` self (`self.K2_GetActorLocation` (`self.PlayerPawn`)) null
    (:`OnSuccess`
      _)
    (:`OnFail`
      _))
  (`self.onMoveToPlayer`))

(fn `UserConstructionScript`)