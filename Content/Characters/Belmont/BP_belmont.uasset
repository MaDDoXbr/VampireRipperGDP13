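; BP_belmont is the player-controlled Belmont character, handling movement, look, jump, sprint and a placeholder shoot through Enhanced Input.
; BeginPlay caches the first player controller and adds the Belmont mapping context, and movement follows that controller's rotation.
; Sprint swaps walk speed and plays or reverses a timeline that blends spring arm length and vertical offset.
; Shoot only plays a pistol montage and prints a debug message.
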(event `self.ReceiveBeginPlay`
  (bind _output_get (set `self.Player0Controller` (`GameplayStatics.GetPlayerController` 0)))
  (`EnhancedInputSubsystemInterface.AddMappingContext` (pcsubsystem `EnhancedInputLocalPlayerSubsystem` _output_get) "/Game/Input/IMC_Belmont.IMC_Belmont" 0 (struct)))

(event `EnhancedInput|/Game/Input/IA_Move`
  (params (ActionValue :type "Vector2D Structure") (ElapsedSeconds :type "Float (double-precision)") (TriggeredSeconds :type "Float (double-precision)") (InputAction :type "InputAction Object Reference" :default "/Game/Input/IA_Move.IA_Move"))
  (bind _player0controller (`self.Player0Controller`))
  (bind (_returnvalue_roll _returnvalue_pitch _returnvalue_yaw) (`KismetMathLibrary.BreakRotator` (`Controller.GetControlRotation` _player0controller)))
  (:`Triggered`
    (`/Engine/EditorBlueprintResources/StandardMacros.IsValid` _player0controller
      (:`Is Valid`
        (`self.AddMovementInput` (`KismetMathLibrary.GetRightVector` (`KismetMathLibrary.MakeRotator` _returnvalue_roll 0.0 _returnvalue_yaw)) ActionValue_X)
        (`self.AddMovementInput` (`KismetMathLibrary.GetForwardVector` (`KismetMathLibrary.MakeRotator` 0.0 0.0 _returnvalue_yaw)) ActionValue_Y)))))

(event `EnhancedInput|/Game/Input/IA_Look`
  (params (ActionValue :type "Vector2D Structure") (ElapsedSeconds :type "Float (double-precision)") (TriggeredSeconds :type "Float (double-precision)") (InputAction :type "InputAction Object Reference" :default "/Game/Input/IA_Look.IA_Look"))
  (:`Triggered`
    (`self.AddControllerYawInput` ActionValue_X)
    (`self.AddControllerPitchInput` ActionValue_Y)))

(event `EnhancedInput|/Game/Input/IA_Jump`
  (params (ActionValue :type Boolean) (ElapsedSeconds :type "Float (double-precision)") (TriggeredSeconds :type "Float (double-precision)") (InputAction :type "InputAction Object Reference" :default "/Game/Input/IA_Jump.IA_Jump"))
  (:`Triggered`
    (`self.Jump`)))

(event `EnhancedInput|/Game/Input/IA_Sprint`
  (params (ActionValue :type Boolean) (ElapsedSeconds :type "Float (double-precision)") (TriggeredSeconds :type "Float (double-precision)") (InputAction :type "InputAction Object Reference" :default "/Game/Input/IA_Sprint.IA_Sprint"))
  (bind _springarm (`self.SpringArm`))
  (:`Triggered`
    (set `CharacterMovementComponent.MaxWalkSpeed` (`self.SprintMoveSpeed`) (`self.CharacterMovement`))
    (bind (_direction _alpha_at_this_frame) (`Timeline|SpringArm Length Timeline` :!label _label)
      (:`Update`
        (set `SpringArmComponent.TargetArmLength` (`KismetMathLibrary.Lerp` (`self.NormalArmLength`) (`self.SprintArmLength`) _alpha_at_this_frame) _springarm)
        (set `SpringArmComponent.TargetOffset` (`KismetMathLibrary.MakeVector` 0.0 0.0 (`KismetMathLibrary.Lerp` (`self.NormalTargetOffset`) (`self.SprintTargetOffset`) _alpha_at_this_frame)) _springarm))))
  (:`Completed`
    (set `CharacterMovementComponent.MaxWalkSpeed` (`self.WalkMoveSpeed`) (`self.CharacterMovement`))
    (goto _label :!via `Reverse`)))

(event `EnhancedInput|/Game/Input/IA_Shoot`
  (params (ActionValue :type Boolean) (ElapsedSeconds :type "Float (double-precision)") (TriggeredSeconds :type "Float (double-precision)") (InputAction :type "InputAction Object Reference" :default "/Game/Input/IA_Shoot.IA_Shoot"))
  (:`Triggered`
    (`|PlayMontage` (`self.Mesh`) "/Game/Characters/Belmont/Animations/Pistol/AM_BM_Pistol_Idle_Montage.AM_BM_Pistol_Idle_Montage"
      (:`then`
        (`KismetSystemLibrary.PrintString` "Anim finished")))))

(fn `UserConstructionScript`)